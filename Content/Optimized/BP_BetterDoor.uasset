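; BP_BetterDoor is a sliding door, single or double, that can open and close automatically as a BP_Body enters or leaves its collision.
; The construction script sets meshes, materials and starting offset from DoorsType, creating a flipped second leaf for double doors.
; Overlap events, gated by AutoDoor, play or reverse timelines that slide the leaves along local Y, mirrored for double doors.
; An OldCode graph retains an earlier stepped-movement approach.
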(event OnComponentEndOverlap(Collision)
  (params (OverlappedComponent :type Primitive%20Component%20Object%20Reference) (OtherActor :type Actor%20Object%20Reference) (OtherComp :type Primitive%20Component%20Object%20Reference) (OtherBodyIndex :type Integer))
  ;[1 1 1] AutoOpenAndColseDoor
  (Utilities|Casting|CastToBP_Body OtherActor)
  (if (Variables|Default|GetAutoDoor)
    (switch Utilities|FlowControl|Switch|SwitchonEDoorsType (Variables|Default|GetDoorsType)
      (:NewEnumerator0
        (CallFunction|CloseSimpleDoor))
      (:NewEnumerator1
        (CallFunction|CloseDoubleDoors)))))

(event OnComponentBeginOverlap(Collision)
  (params (OverlappedComponent :type Primitive%20Component%20Object%20Reference) (OtherActor :type Actor%20Object%20Reference) (OtherComp :type Primitive%20Component%20Object%20Reference) (OtherBodyIndex :type Integer) (bFromSweep :type Boolean) (SweepResult :type Hit%20Result%20Structure%20%28by%20ref%29))
  ;[1 1 1] AutoOpenAndColseDoor
  (Utilities|Casting|CastToBP_Body OtherActor)
  (if (Variables|Default|GetAutoDoor)
    (switch Utilities|FlowControl|Switch|SwitchonEDoorsType (Variables|Default|GetDoorsType)
      (:NewEnumerator0
        (CallFunction|OpenSimpleDoor))
      (:NewEnumerator1
        (CallFunction|OpenDoubleDoors)))))

(event Custom|CloseSimpleDoor
  ;[1 1 1] AutoOpenAndColseDoor
  (bind _open_closedoors (Timeline|TL_SimpleDoor Reverse)
    (:Update
      (Transformation|SetRelativeLocation (Variables|Default|GetDoor01) (Math|Vector|MakeVector 0.0 (* 1e+02 _open_closedoors) 0.0) false false))))

(event Custom|OpenSimpleDoor
  ;[1 1 1] AutoOpenAndColseDoor
  (bind _open_closedoors (Timeline|TL_SimpleDoor Play)
    (:Update
      (Transformation|SetRelativeLocation (Variables|Default|GetDoor01) (Math|Vector|MakeVector 0.0 (* 1e+02 _open_closedoors) 0.0) false false))))

(event Custom|CloseDoubleDoors
  ;[1 1 1] AutoOpenAndColseDoor
  (bind _open_closedoors (Timeline|TL_DoubleDoors Reverse)
    (:Update
      (Transformation|SetRelativeLocation (Variables|Default|GetDoor01) (Math|Vector|MakeVector 0.0 (* 1e+02 _open_closedoors) 0.0) false false)
      (Transformation|SetRelativeLocation (Variables|Default|GetDoor2) (Math|Vector|MakeVector 0.0 (* (* 1e+02 _open_closedoors) -1.0) 0.0) false false))))

(event Custom|OpenDoubleDoors
  ;[1 1 1] AutoOpenAndColseDoor
  (bind _open_closedoors (Timeline|TL_DoubleDoors Play)
    (:Update
      (Transformation|SetRelativeLocation (Variables|Default|GetDoor01) (Math|Vector|MakeVector 0.0 (* 1e+02 _open_closedoors) 0.0) false false)
      (Transformation|SetRelativeLocation (Variables|Default|GetDoor2) (Math|Vector|MakeVector 0.0 (* (* 1e+02 _open_closedoors) -1.0) 0.0) false false))))

(fn ConstructionScript
  (bind _materail2 (Variables|Default|GetMaterail2))
  (bind _doorjamb (Variables|Default|GetDoorJamb))
  (bind _doorposition (Variables|Default|GetDoorPosition))
  (bind _materail1 (Variables|Default|GetMaterail1))
  (bind _doorjamb_2 (Variables|Default|GetDoorJamb))
  (switch Utilities|FlowControl|Switch|SwitchonEDoorsType (Variables|Default|GetDoorsType)
    (:NewEnumerator0
      ;[1 1 1] SimpleDoor
      (Components|StaticMesh|SetStaticMesh (Variables|Default|GetDoor01) (Variables|Default|GetSM_Door1))
      (Components|StaticMesh|SetStaticMesh (Variables|Default|GetDoorJamb) (Variables|Default|GetSM_DoorJamb))
      (Utilities|IsValid (Variables|Default|GetDoor2)
        (:Is%20Valid
          (Components|DestroyComponent (Variables|Default|GetDoor2)))
        (:Is%20Not%20Valid
          _))
      (Transformation|AddRelativeLocation (Variables|Default|GetDoor01) (Math|Vector|MakeVector 0.0 (Variables|Default|GetDoorPosition) 0.0) false false)
      (Rendering|Material|SetMaterial _doorjamb_2 0 (Variables|Default|GetMaterail1))
      (Rendering|Material|SetMaterial _doorjamb_2 1 (Variables|Default|GetMaterail2)))
    (:NewEnumerator1
      (Components|StaticMesh|SetStaticMesh (Variables|Default|GetDoor01) (Variables|Default|GetSM_Door1))
      (Components|StaticMesh|SetStaticMesh (Variables|Default|GetDoorJamb) (Variables|Default|GetSM_DoorJamb))
      (bind _returnvalue (AddComponent|AddStaticMeshComponent false))
      (Components|StaticMesh|SetStaticMesh _returnvalue (Variables|Default|GetSM_Door2))
      (Transformation|SetRelativeRotation _returnvalue "0.000000,180.000000,0.000000" false false)
      (Variables|Default|SetDoor2 _returnvalue)
      (Transformation|AddRelativeLocation (Variables|Default|GetDoor01) (Math|Vector|MakeVector 0.0 _doorposition 0.0) false false)
      (Transformation|AddRelativeLocation (Variables|Default|GetDoor2) (Math|Vector|MakeVector 0.0 (* _doorposition -1.0) 0.0) false false)
      (Rendering|Material|SetMaterial _doorjamb 0 _materail1)
      (Rendering|Material|SetMaterial _doorjamb 1 _materail2)
      (Rendering|Material|SetMaterial (Variables|Default|GetDoor2) 0 _materail2)
      (Rendering|Material|SetMaterial (Variables|Default|GetDoor2) 1 _materail1)
      (Rendering|Material|SetMaterial (Variables|Default|GetDoor01) 2 (Variables|Default|GetMaterail3)))))

(fn OldCode
  (if (Variables|Default|GetAutoDoor)
    (if true
      (Math|Float|CompareFloat (Variables|Default|GetDoorPosition) 105.0
        (:>
          (Variables|Default|SetDoorPosition 105.0 :!label _label))
        (:==
          (goto _label))
        (:<
          (Variables|Default|SetDoorPosition (+ (Variables|Default|GetDoorPosition) 3.0))
          (Transformation|SetRelativeLocation (Variables|Default|GetDoor01) (Math|Vector|MakeVector 0.0 (Variables|Default|GetDoorPosition) 0.0) false false :!label _label_2)))
      (elif true
        (Math|Float|CompareFloat (Variables|Default|GetDoorPosition) 0.0
          (:>
            (Variables|Default|SetDoorPosition (- (Variables|Default|GetDoorPosition) 3.0))
            (goto _label_2))
          (:==
            _)
          (:<
            _))
        (Variables|Default|SetDoorPosition 0.0)))))