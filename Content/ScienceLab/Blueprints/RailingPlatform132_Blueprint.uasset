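; Railing platform Blueprint for the ScienceLab that controls whether its static meshes simulate physics.
; The construction script turns physics simulation off on the main mesh component.
; CheckWorldGravity, not called within this graph, sets simulation on every static mesh component by comparing chopped string text to "-980".
; That parse starts from an empty string rather than reading world gravity, and the descriptive gravity literal is unconnected.
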(fn ConstructionScript
  (Physics|SetSimulatePhysics (Variables|Default|GetRailingPlatform132_StaticMeshComponent0) false))

(fn CheckWorldGravity
  ;[1 0 0] Compute -9.8m/s
  (for _array_element (Actor|GetComponentsByClass "/Script/Engine.StaticMeshComponent")
    (bind _asstatic_mesh_component (Utilities|Casting|CastToStaticMeshComponent _array_element))
    (Physics|SetSimulatePhysics _asstatic_mesh_component (== (Utilities|String|LeftChop (.RightS (Utilities|String|Split "" (Utilities|String|GetSubstring "" 44 2))) 33) "-980"))))